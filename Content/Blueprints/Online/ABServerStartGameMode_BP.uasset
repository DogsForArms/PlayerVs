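; Game mode for a dedicated server's startup map that registers an online session and then travels to the configured map.
; On BeginPlay, dedicated servers only, it parses server name, game mode and map from the command line and prints them for debug.
; It creates an Advanced Session with the server name as GAMENAME.
; On success it opens the map with listen, game and hardcoded MinimumPlayers options.
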(event `self.ReceiveBeginPlay`
  (bind (_returnvalue_servername _returnvalue_game _returnvalue_map) (break `GameConfig` (`self.ParseGameConfigFromCommandLine`)))
  (if (`KismetSystemLibrary.IsDedicatedServer`)
    (`KismetSystemLibrary.PrintString` (`KismetStringLibrary.Concat_StrStr` "DEBUG BP serverName: " (`KismetStringLibrary.Conv_NameToString` _returnvalue_servername) "|game: " (`KismetStringLibrary.Conv_NameToString` _returnvalue_game) "|MapName" (`KismetStringLibrary.Conv_NameToString` _returnvalue_map)))
    (`CreateSessionCallbackProxyAdvanced.CreateAdvancedSession` (`|MakeArray` (`AdvancedSessionsLibrary.MakeLiteralSessionPropertyString` "GAMENAME" (`KismetStringLibrary.Conv_NameToString` _returnvalue_servername))) (`GameplayStatics.GetPlayerController` 0) 8 8 false true true false
      (:`OnSuccess`
        (`GameplayStatics.OpenLevel` _returnvalue_map true (`KismetStringLibrary.Concat_StrStr` "listen" "?game=" (`KismetStringLibrary.Conv_NameToString` _returnvalue_game) "?MinimumPlayers=" "2"))))))

(fn `UserConstructionScript`)