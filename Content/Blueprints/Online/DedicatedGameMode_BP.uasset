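; Dedicated server game mode that bootstraps an online match from command-line configuration.
; On BeginPlay it prints the parsed config for debugging, then creates an 8-slot Advanced Session flagged as dedicated, publishing the server name as GAMENAME.
; On success it opens the configured map as a listen level, passing game mode, player limits, round time and match timings as URL options.
; Session failure has no handling.
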(event `self.ReceiveBeginPlay`
  (bind (_returnvalue_servername _returnvalue_game _returnvalue_map _returnvalue_roundtime _returnvalue_minimumplayers _returnvalue_maximumplayers _returnvalue_timebetweenmatches _returnvalue_timebeforematch) (break `GameConfig` (`self.ParseGameConfigFromCommandLine`)))
  (bind _returnvalue (`KismetStringLibrary.Conv_IntToString` _returnvalue_roundtime))
  (`KismetSystemLibrary.PrintString` (`KismetStringLibrary.Concat_StrStr` "DEBUG BP serverName: " _returnvalue_servername "|game: " _returnvalue_game "|MapName" _returnvalue_map "|RoundTime: " _returnvalue) true true (struct :`G` 0.66 :`B` 1.0 :`A` 1.0) 20.0)
  (`CreateSessionCallbackProxyAdvanced.CreateAdvancedSession` (`|MakeArray` (`AdvancedSessionsLibrary.MakeLiteralSessionPropertyString` "GAMENAME" _returnvalue_servername)) (`GameplayStatics.GetPlayerController` 0) 8 8 false true true false
    (:`OnSuccess`
      (`GameplayStatics.OpenLevel` (`KismetStringLibrary.Conv_StringToName` _returnvalue_map) true (`KismetStringLibrary.Concat_StrStr` "listen" "?game=" _returnvalue_game "?MinimumPlayers=" (`KismetStringLibrary.Conv_IntToString` _returnvalue_minimumplayers) "?MaximumPlayers=" (`KismetStringLibrary.Conv_IntToString` _returnvalue_maximumplayers) "?RoundTime=" _returnvalue "?TimeBetweenMatches=" (`KismetStringLibrary.Conv_IntToString` _returnvalue_timebetweenmatches) "?TimeBeforeMatch=" (`KismetStringLibrary.Conv_IntToString` _returnvalue_timebeforematch))))))

(fn `UserConstructionScript`)