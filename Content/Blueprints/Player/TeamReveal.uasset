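; TeamReveal is a player-attached indicator actor that shows a character's team in the TTT mode once that team is revealed.
; On BeginPlay it finds the parent character's player state, creates a dynamic material for its static mesh and binds to the team reveal event.
; On reveal it sets the material's team color and shows the mesh for Alien or Innocent, hiding it for Unassigned.
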(event `self.ReceiveBeginPlay`
  (bind _asabcharacter (cast `ABCharacter` (`self.GetParentActor`)))
  (bind _asabtttplayer_state (cast `ABTTTPlayerState` (`Pawn.PlayerState` _asabcharacter)))
  (`|ExecutionSequence`
    (:`then_0`
      ;[1 1 1] dynamic material instance
      (bind _returnvalue (`PrimitiveComponent.CreateDynamicMaterialInstance` (`self.StaticMesh`) 0 null "None"))
      (bind _output_get (set `self.DynamicMaterial` _returnvalue))
      (`PrimitiveComponent.SetMaterial` (`self.StaticMesh`) 0 _output_get))
    (:`then_1`
      (add `ABTTTPlayerState.OnTeamReveal` _asabtttplayer_state (delegate `OnTeamReveal`)))))

(event `OnTeamReveal`
  (params (team :type "ETeam Enum" :default "Unassigned"))
  (`MaterialInstanceDynamic.SetVectorParameterValue` (`self.DynamicMaterial`) "TeamColor" (select `ETeam` team :`Unassigned` (struct :`R` 1.0 :`G` 1.0 :`B` 1.0 :`A` 1.0) :`Alien` (struct :`R` 1.0 :`B` 0.042602 :`A` 1.0) :`Innocent` (struct :`G` 1.0 :`B` 0.090115 :`A` 1.0) :!type "LinearColor Structure"))
  (`SceneComponent.SetVisibility` (`self.StaticMesh`) (select `ETeam` team :`Alien` true :`Innocent` true) true))

(fn `UserConstructionScript`)