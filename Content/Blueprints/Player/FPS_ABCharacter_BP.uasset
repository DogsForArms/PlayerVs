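; FPS player character that adapts a VR character Blueprint for first-person play with standard axis input.
; On BeginPlay it attaches both motion controllers to the replicated VR camera and loads the FPS_Pawn controller profile.
; It removes the camera as a tick prerequisite of the controllers to fix physics delay from the attachment.
; Turn and LookUp drive controller yaw and pitch, while Forward and Right move along VR-relative vectors.
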(event `self.ReceiveBeginPlay`
  (bind _vrreplicatedcamera (`self.VRReplicatedCamera`))
  (bind _vrreplicatedcamera_2 (`self.VRReplicatedCamera`))
  (`parent.ReceiveBeginPlay`)
  ;[1 1 1] VR to FPS Setup
  (`SceneComponent.K2_AttachToComponent` (`self.LeftMotionController`) _vrreplicatedcamera_2 "None" "KeepRelative" "KeepRelative" "KeepRelative" true)
  (`SceneComponent.K2_AttachToComponent` (`self.RightMotionController`) _vrreplicatedcamera_2 "None" "KeepRelative" "KeepRelative" "KeepRelative" true)
  (`VRGlobalSettings.LoadControllerProfileByName` "FPS_Pawn")
  ;;[1 1 1] Fixes physics delay from attachment
  (`ActorComponent.RemoveTickPrerequisiteComponent` (`self.LeftMotionController`) _vrreplicatedcamera)
  (`ActorComponent.RemoveTickPrerequisiteComponent` (`self.RightMotionController`) _vrreplicatedcamera))

(event `InputAxis|Turn`
  (params (AxisValue :type "Float (single-precision)"))
  ;[1 1 1] Movement & Look
  (`self.AddControllerYawInput` AxisValue))

(event `InputAxis|LookUp`
  (params (AxisValue :type "Float (single-precision)"))
  ;[1 1 1] Movement & Look
  (`self.AddControllerPitchInput` AxisValue))

(event `InputAxis|Forward`
  (params (AxisValue :type "Float (single-precision)"))
  ;[1 1 1] Movement & Look
  (`self.AddMovementInput` (`self.GetVRForwardVector`) AxisValue))

(event `InputAxis|Right`
  (params (AxisValue :type "Float (single-precision)"))
  ;[1 1 1] Movement & Look
  (`self.AddMovementInput` (`self.GetVRRightVector`) AxisValue))

(fn `UserConstructionScript`
  (`parent.UserConstructionScript`))