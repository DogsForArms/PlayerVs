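; Player VR character Blueprint that hands its motion controllers to C++ and sets up positional voice chat.
; On BeginPlay it passes both controllers and their grab spheres to InitializeHands, then sets game-only input on its player controller.
; VOIP setup polls in a delay loop until PlayerState is valid, then registers the talker and attaches attenuated voice to the replicated VR camera.
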(event `self.ReceiveBeginPlay`
  (bind _voiptalker (`self.VOIPTalker`))
  (`|ExecutionSequence`
    (:`then_0`
      ;[1 1 1] BP -> C++ Initialization
      (`self.InitializeHands` (`self.LeftMotionController`) (`self.RightMotionController`) (`self.LeftSphere`) (`self.RightSphere`)))
    (:`then_1`
      ;[1 1 1] VOIP Settings
      (`/Engine/EditorBlueprintResources/StandardMacros.IsValid` (`self.PlayerState`) :!label _label
        (:`Is Valid`
          (`KismetSystemLibrary.Delay` 0.2)
          (`VOIPTalker.RegisterWithPlayerState` _voiptalker (`self.PlayerState`))
          (set `VOIPTalker.Settings` (make `VoiceSettings` (`self.VRReplicatedCamera`) "/Game/Blueprints/Player/VOIPAttenuation.VOIPAttenuation") _voiptalker))
        (:`Is Not Valid`
          ;;[1 0.1607 0] retry
          (`KismetSystemLibrary.PrintString` "VOIP setup Delay (waiting for player state)" false)
          (`KismetSystemLibrary.Delay` 0.1)
          (goto _label))))
    (:`then_2`
      (`WidgetBlueprintLibrary.SetInputMode_GameOnly` (cast `PlayerController` (`self.GetController`) :!pure true)))))

(fn `UserConstructionScript`)